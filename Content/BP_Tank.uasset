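; BP_Tank is an actor that periodically teleports to a random spot within a large flat square centred on the world origin.
; Tick starts a one-shot 15-second timer whenever the stored handle is invalid.
; When it fires, SetRandomLocation moves the actor without sweeping, at a fixed height, then invalidates the handle so Tick re-arms the timer.
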(event `self.ReceiveTick`
  (params (DeltaSeconds :type "Float (single-precision)"))
  (if (not (`KismetSystemLibrary.K2_IsValidTimerHandle` (`self.Timer`)))
    (bind _returnvalue (`KismetSystemLibrary.K2_SetTimerDelegate` (delegate `SetRandomLocation`) 15.0))
    (set `self.Timer` _returnvalue)))

(event `SetRandomLocation`
  (`self.K2_SetActorLocation` (`KismetMathLibrary.RandomPointInBoundingBox` (`KismetMathLibrary.MakeVector` 0.0 0.0 36.092216) (`KismetMathLibrary.MakeVector` 9000.0 9000.0 0.0)) false true)
  (`KismetSystemLibrary.K2_InvalidateTimerHandle` (`self.Timer`)))

(fn `UserConstructionScript`)